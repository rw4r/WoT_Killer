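; Player tank Blueprint that routes input to driving, camera rotation and firing.
; On BeginPlay it hands barrel and turret to TankAiming and both tracks to TankMovement.
; Driving supports direct per-track throttle or turn and accelerate intents through TankMovement, with Reverse sharing the accelerate call.
; Azimuth yaws a Scene component and Elevation pitches the SpringArm, both scaled by delta time, while Fire calls a function defined outside these graphs.
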(event `self.ReceiveBeginPlay`
  (`TankAimingComponent.Initialize` (`self.TankAiming`) (`self.Barrel`) (`self.Turret`))
  (`TankMovementComponent.Initialize` (`self.TankMovement`) (`self.Track_Left`) (`self.Track_Right`)))

(event `InputAction|Fire`
  (params (Key :type "Key Structure" :default "AnyKey"))
  (:`Pressed`
    (`self.Fire`)))

(event `InputAxis|Throttle_Right`
  (params (AxisValue :type "Float (single-precision)"))
  ;[1 1 1] Movement Input Binding
  (`TankTrack.SetThrottle` (`self.Track_Right`) AxisValue))

(event `InputAxis|Azimuth`
  (params (AxisValue :type "Float (single-precision)"))
  ;[1 1 1] Aim Input Binding
  (`SceneComponent.K2_AddLocalRotation` (`self.Scene`) (`KismetMathLibrary.MakeRotator` 0.0 0.0 (* AxisValue (`GameplayStatics.GetWorldDeltaSeconds`) 100.0)) false false))

(event `InputAxis|Throttle_Left`
  (params (AxisValue :type "Float (single-precision)"))
  ;[1 1 1] Movement Input Binding
  (`TankTrack.SetThrottle` (`self.Track_Left`) AxisValue))

(event `InputAxis|Turn_Right`
  (params (AxisValue :type "Float (single-precision)"))
  ;[1 1 1] Movement Input Binding
  (`TankMovementComponent.IntendTurnRight` (`self.TankMovement`) AxisValue))

(event `InputAxis|Accelerate`
  (params (AxisValue :type "Float (single-precision)"))
  ;[1 1 1] Movement Input Binding
  (`TankMovementComponent.IntendAccelerate` (`self.TankMovement`) AxisValue))

(event `InputAxis|Turn_Left`
  (params (AxisValue :type "Float (single-precision)"))
  ;[1 1 1] Movement Input Binding
  (`TankMovementComponent.IntendTurnLeft` (`self.TankMovement`) AxisValue))

(event `InputAxis|Reverse`
  (params (AxisValue :type "Float (single-precision)"))
  ;[1 1 1] Movement Input Binding
  (`TankMovementComponent.IntendAccelerate` (`self.TankMovement`) AxisValue))

(event `InputAxis|Elevation`
  (params (AxisValue :type "Float (single-precision)"))
  ;[1 1 1] Aim Input Binding
  (`SceneComponent.K2_AddLocalRotation` (`self.SpringArm`) (`KismetMathLibrary.MakeRotator` 0.0 (* (`GameplayStatics.GetWorldDeltaSeconds`) AxisValue 100.0)) false false))

(fn `UserConstructionScript`)